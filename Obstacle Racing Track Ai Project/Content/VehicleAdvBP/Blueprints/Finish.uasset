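; Finish line actor for an AI vehicle race that detects cars crossing its box trigger and declares the race finished.
; A per-vehicle CanPass array, indexed by vehicle Id, decides whether a crossing counts as a finish or instead unlocks the linked next checkpoint for that car.
; Each valid finish prints the controller's team name, while only the first sets the game mode's Semaphore text to announce the end.
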(event OnComponentBeginOverlap(Box)
  (params (OverlappedComponent :type Primitive%20Component%20Object%20Reference) (OtherActor :type Actor%20Object%20Reference) (OtherComp :type Primitive%20Component%20Object%20Reference) (OtherBodyIndex :type Integer) (bFromSweep :type Boolean) (SweepResult :type Hit%20Result%20Structure%20%28by%20ref%29))
  (bind _asaivehicle (Utilities|Casting|CastToAIVehicle OtherActor))
  (if (Utilities|Array|Get(acopy) (Variables|Default|GetbCanPass) (Variables|/Game/AI/AIVehicle.AIVehicle_C|GetId _asaivehicle))
    (Development|PrintString (Utilities|String|ToString(Text) (Variables|/Game/AI/CarController.CarController_C|GetTeamName (.AsCar%20Controller (Utilities|Casting|CastToCarController (AI|GetAIController _asaivehicle))))))
    (if (not (Variables|Default|GetbTresspassed))
      (Variables|Default|SetbTresspassed true)
      (Variables|/Game/VehicleAdvBP/Blueprints/VehicleAdvGameMode.VehicleAdvGameMode_C|SetSemaphore (.AsVehicle%20Adv%20Game%20Mode (Utilities|Casting|CastToVehicleAdvGameMode (Game|GetGameMode))) "Race Finished!!!"))
    (else
      (Utilities|Array|SetArrayElem (Variables|/Game/VehicleAdvBP/Blueprints/Checkpoint.Checkpoint_C|GetbCanPass (Variables|Default|GetNextCheckpoint)) (Variables|/Game/AI/AIVehicle.AIVehicle_C|GetId _asaivehicle) true))))

(event Collision|EventActorBeginOverlap
  (params (OtherActor :type Actor%20Object%20Reference))
  (|CallParentFunction OtherActor) ; This node is disabled and will not be called.\nDrag off pins to build functionality.
)

(event EventTick
  (params (DeltaSeconds :type Float%20%28single-precision%29))
  (|CallParentFunction DeltaSeconds) ; This node is disabled and will not be called.\nDrag off pins to build functionality.
)

(fn ConstructionScript
  (|CallParentFunction))