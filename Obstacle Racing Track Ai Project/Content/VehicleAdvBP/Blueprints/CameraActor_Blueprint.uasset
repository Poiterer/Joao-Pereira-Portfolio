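; Camera actor Blueprint that provides a top-down follow view of the leading car in the vehicle game.
; Each tick it reads BestCar from VehicleAdvGameMode, falling back to the first car controller's pawn when that is invalid.
; It eases the camera component toward a point high above that car using a frame-time-scaled lerp, changing location only.
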(event EventTick
  (params (DeltaSeconds :type Float%20%28single-precision%29))
  (bind _returnvalue (Game|GetGameMode))
  (bind _cameracomponent (Variables|CameraActor|GetCameraComponent))
  (bind _asvehicle_adv_game_mode (Utilities|Casting|CastToVehicleAdvGameMode _returnvalue))
  (bind _bestcar (Variables|/Game/VehicleAdvBP/Blueprints/VehicleAdvGameMode.VehicleAdvGameMode_C|GetBestCar _asvehicle_adv_game_mode))
  (Transformation|SetWorldLocation _cameracomponent (Math|Vector|Lerp(Vector) (Transformation|GetWorldLocation _cameracomponent) (+ (Transformation|GetActorLocation (select (Utilities|IsValid _bestcar) _bestcar (Pawn|GetControlledPawn (Utilities|Array|Get(acopy) (Variables|/Game/VehicleAdvBP/Blueprints/VehicleAdvGameMode.VehicleAdvGameMode_C|GetCarControllers _asvehicle_adv_game_mode))))) "0, 0,1250.000000") (* DeltaSeconds 5.0)) false false))

(fn ConstructionScript)