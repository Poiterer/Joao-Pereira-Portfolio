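; Checkpoint actor that tracks AI vehicle progress through a linked chain of checkpoints and reports the leading car.
; When an AIVehicle permitted by this checkpoint's CanPass array overlaps the Box, it unlocks NextCheckpoint for that vehicle's Id, enforcing order.
; The first permitted vehicle through sets the one-time Tresspassed flag and becomes BestCar on VehicleAdvGameMode.
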(event OnComponentBeginOverlap(Box)
  (params (OverlappedComponent :type Primitive%20Component%20Object%20Reference) (OtherActor :type Actor%20Object%20Reference) (OtherComp :type Primitive%20Component%20Object%20Reference) (OtherBodyIndex :type Integer) (bFromSweep :type Boolean) (SweepResult :type Hit%20Result%20Structure%20%28by%20ref%29))
  (bind _asaivehicle (Utilities|Casting|CastToAIVehicle OtherActor))
  (if (Utilities|Array|Get(acopy) (Variables|Default|GetbCanPass) (Variables|/Game/AI/AIVehicle.AIVehicle_C|GetId _asaivehicle))
    (Utilities|Array|SetArrayElem (Variables|Checkpoint_C|GetbCanPass (Variables|Default|GetNextCheckpoint)) (Variables|/Game/AI/AIVehicle.AIVehicle_C|GetId _asaivehicle) true true)
    (if (not (Variables|Default|GetbTresspassed))
      (Variables|Default|SetbTresspassed true)
      (Variables|/Game/VehicleAdvBP/Blueprints/VehicleAdvGameMode.VehicleAdvGameMode_C|SetBestCar (.AsVehicle%20Adv%20Game%20Mode (Utilities|Casting|CastToVehicleAdvGameMode (Game|GetGameMode))) _asaivehicle))))

(event EventBeginPlay)

(event Collision|EventActorBeginOverlap
  (params (OtherActor :type Actor%20Object%20Reference)))

(event EventTick
  (params (DeltaSeconds :type Float%20%28single-precision%29)))

(fn ConstructionScript)